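; BP_FPS_Character is a first-person character Blueprint that handles basic player movement, camera look and jumping.
; Axis inputs feed controller yaw and pitch for looking, and movement input along the capsule component's forward and right vectors.
; The Jump action calls the character's Jump on press, while BeginPlay, Tick, overlap and the construction script hold no logic.
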(event `InputAxis|Turn`
  (params (AxisValue :type "Float (single-precision)"))
  ; Camera
  (`self.AddControllerYawInput` AxisValue))

(event `InputAxis|Move Forward`
  (params (AxisValue :type "Float (single-precision)"))
  ; Movement
  (`self.AddMovementInput` (`SceneComponent.GetForwardVector` (`self.CapsuleComponent`)) AxisValue))

(event `InputAction|Jump`
  (params (Key :type "Key Structure"))
  ; Action Mappings
  (:`Pressed`
    (`self.Jump`)))

(event `InputAxis|Look Up`
  (params (AxisValue :type "Float (single-precision)"))
  ; Camera
  (`self.AddControllerPitchInput` AxisValue))

(event `InputAxis|Move Right`
  (params (AxisValue :type "Float (single-precision)"))
  ; Movement
  (`self.AddMovementInput` (`SceneComponent.GetRightVector` (`self.CapsuleComponent`)) AxisValue))

(fn `UserConstructionScript`)